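; BP_CameraFollow is a fixed-position camera that takes over the player's view while BP_CameraCharacter is inside its Box trigger.
; Overlapping Box blends the view target to this actor, and leaving blends it back to the character.
; Each Tick eases the camera toward the player with a fixed-alpha, frame-rate-dependent rotator lerp, clamping yaw to a narrow arc.
; A second Box_View trigger plays or reverses an FOV zoom timeline when CanZoom is set.
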(event OnComponentBeginOverlap(Box)
  (params (OverlappedComponent :type Primitive%20Component%20Object%20Reference) (OtherActor :type Actor%20Object%20Reference) (OtherComp :type Primitive%20Component%20Object%20Reference) (OtherBodyIndex :type Integer) (bFromSweep :type Boolean) (SweepResult :type Hit%20Result%20Structure%20%28by%20ref%29))
  ;[0.15 0.15 0.15 0.5] Set View Target
  (Utilities|Casting|CastToBP_CameraCharacter OtherActor)
  (Game|Player|SetViewTargetwithBlend (Game|GetPlayerController 0) self 2.0 "VTBlend_Linear" 1.0 true))

(event OnComponentEndOverlap(Box)
  (params (OverlappedComponent :type Primitive%20Component%20Object%20Reference) (OtherActor :type Actor%20Object%20Reference) (OtherComp :type Primitive%20Component%20Object%20Reference) (OtherBodyIndex :type Integer))
  ;[0.15 0.15 0.15 0.5] Set View Target
  (bind _asbp_third_person_character (Utilities|Casting|CastToBP_CameraCharacter OtherActor))
  (Game|Player|SetViewTargetwithBlend (Game|GetPlayerController 0) _asbp_third_person_character 2.0 "VTBlend_Linear" 1.0 true))

(event OnComponentBeginOverlap(Box_View)
  (params (OverlappedComponent :type Primitive%20Component%20Object%20Reference) (OtherActor :type Actor%20Object%20Reference) (OtherComp :type Primitive%20Component%20Object%20Reference) (OtherBodyIndex :type Integer) (bFromSweep :type Boolean) (SweepResult :type Hit%20Result%20Structure%20%28by%20ref%29))
  ;[0.15 0.15 0.15 0.5] Overlap Player
  (Utilities|Casting|CastToBP_CameraCharacter OtherActor)
  (CallFunction|Zoomin))

(event OnComponentEndOverlap(Box_View)
  (params (OverlappedComponent :type Primitive%20Component%20Object%20Reference) (OtherActor :type Actor%20Object%20Reference) (OtherComp :type Primitive%20Component%20Object%20Reference) (OtherBodyIndex :type Integer))
  ;[0.15 0.15 0.15 0.5] Overlap Player
  (Utilities|Casting|CastToBP_CameraCharacter OtherActor)
  (CallFunction|ZoomOut))

(event Custom|RotationOnPlayer
  (bind _returnvalue (Game|Player|GetPlayerPawn 0))
  (bind _camera (Variables|Default|GetCamera))
  (bind _camera_2 (Variables|Default|GetCamera))
  (bind _returnvalue_2 (Transformation|GetWorldRotation _camera_2))
  (bind _returnvalue_3 (Transformation|GetActorTransform _returnvalue))
  (bind _returnvalue_4 (Transformation|GetWorldLocation _camera))
  (bind _returnvalue_5 (Math|Rotator|FindLookatRotation _returnvalue_4 (.location _returnvalue_3)))
  (bind _returnvalue_6 (Math|Rotator|Lerp(Rotator) _returnvalue_2 _returnvalue_5 0.01))
  ;[0.15 0.15 0.15 0.5] Camera Look on Player
  (Transformation|SetWorldRotation _camera (Math|Rotator|MakeRotator (.roll _returnvalue_6) (.pitch _returnvalue_6) (Math|Float|Clamp(Float) (.yaw _returnvalue_6) -105.0 -75.0)) false false))

(event Custom|ZoomIn
  ;[0.15 0.15 0.15 0.5] Camera field of view
  (if (Variables|Default|GetCanZoom)
    (bind _newtrack_0 (Timeline|Timeline Play)
      (:Update
        (Camera|SetFieldOfView (Variables|Default|GetCamera) _newtrack_0)))))

(event Custom|ZoomOut
  ;[0.15 0.15 0.15 0.5] Camera field of view
  (if (Variables|Default|GetCanZoom)
    (bind _newtrack_0 (Timeline|Timeline Reverse)
      (:Update
        (Camera|SetFieldOfView (Variables|Default|GetCamera) _newtrack_0)))))

(event EventTick
  (params (DeltaSeconds :type Float%20%28single-precision%29))
  (CallFunction|RotationonPlayer))

(fn ConstructionScript)