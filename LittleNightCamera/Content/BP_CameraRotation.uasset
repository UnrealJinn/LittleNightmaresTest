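; BP_CameraRotation is a trigger volume that rotates the third-person character's camera boom as the player enters and leaves its box.
; BeginPlay caches the player's CameraBoom.
; Begin overlap stops rotation on every BP_CameraRotation actor, then moves the boom toward the front rotation; end overlap moves it toward the back rotation.
; Both timed MoveComponentTo rotations are gated by CanRotate.
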(event OnComponentBeginOverlap(Box)
  (params (OverlappedComponent :type Primitive%20Component%20Object%20Reference) (OtherActor :type Actor%20Object%20Reference) (OtherComp :type Primitive%20Component%20Object%20Reference) (OtherBodyIndex :type Integer) (bFromSweep :type Boolean) (SweepResult :type Hit%20Result%20Structure%20%28by%20ref%29))
  (Utilities|Casting|CastToBP_ThirdPersonCharacter OtherActor)
  (Utilities|FlowControl|Sequence
    (:then_0
      (bind _outactors (Actor|GetAllActorsOfClass "BP_CameraRotation_C"))
      (for _array_element _outactors
        (Utilities|IsValid _array_element
          (:Is%20Valid
            (CallFunction|StopRotation _array_element)))))
    (:then_1
      (CallFunction|RotateFront))))

(event OnComponentEndOverlap(Box)
  (params (OverlappedComponent :type Primitive%20Component%20Object%20Reference) (OtherActor :type Actor%20Object%20Reference) (OtherComp :type Primitive%20Component%20Object%20Reference) (OtherBodyIndex :type Integer))
  (Utilities|Casting|CastToBP_ThirdPersonCharacter OtherActor)
  (CallFunction|RotateBack))

(event Custom|Rotate_Front
  (if (Variables|Default|GetCanRotate)
    (Components|MoveComponentTo (Variables|Default|GetCamera%20Boom) "0, 0, 0" (Variables|Default|GetRotateFront) false false (Variables|Default|GetRotationSpeed) false)))

(event Custom|Rotate_Back
  (if (Variables|Default|GetCanRotate)
    (Components|MoveComponentTo (Variables|Default|GetCamera%20Boom) "0, 0, 0" (Variables|Default|GetRotateBack) false false (Variables|Default|GetRotationSpeed) false)))

(event Custom|Stop%20Rotation
  (Components|MoveComponentTo (Variables|Default|GetCamera%20Boom) "0, 0, 0" (Variables|Default|GetRotateBack) false false (Variables|Default|GetRotationSpeed) false) ; enters at Stop
)

(event EventBeginPlay
  (bind _asbp_third_person_character (Utilities|Casting|CastToBP_ThirdPersonCharacter (Game|GetPlayerCharacter 0)))
  (Variables|Default|SetCamera%20Boom (Variables|/Game/ThirdPerson/Blueprints/BP_ThirdPersonCharacter.BP_ThirdPersonCharacter_C|GetCameraBoom _asbp_third_person_character)))

(fn ConstructionScript)